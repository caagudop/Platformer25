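; BP_Elevator is a platform the player ball raises with the Action input while inside its trigger.
; The trigger toggles input and the HUD interaction prompt, using a HUD reference cached from BP_PlayerBall after a startup delay.
; Leaving the trigger automatically sends the platform down.
; Tick moves it vertically by a fixed per-frame step, without delta-time scaling or sweep, stopping once it reaches the upper or lower limit.
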(event `self.ReceiveBeginPlay`
  (`KismetSystemLibrary.Delay` 2.0)
  (bind _asbp_player_ball (cast `/Game/Blueprints/BP_PlayerBall` (`GameplayStatics.GetPlayerPawn` 0)))
  (set `self.UIHUDREF` (`/Game/Blueprints/BP_PlayerBall.HUD REF` _asbp_player_ball)))

(event `self.Trigger.OnComponentBeginOverlap`
  (params (OverlappedComponent :type "PrimitiveComponent Object Reference") (OtherActor :type "Actor Object Reference") (OtherComp :type "PrimitiveComponent Object Reference") (OtherBodyIndex :type Integer) (bFromSweep :type Boolean) (SweepResult :type "HitResult Structure (by ref)"))
  (cast `/Game/Blueprints/BP_PlayerBall` OtherActor)
  (`self.EnableInput` (`GameplayStatics.GetPlayerController` 0))
  (`/Game/HUD/HUD_Principal.ShowInteractionText` (`self.UIHUDREF`)))

(event `self.Trigger.OnComponentEndOverlap`
  (params (OverlappedComponent :type "PrimitiveComponent Object Reference") (OtherActor :type "Actor Object Reference") (OtherComp :type "PrimitiveComponent Object Reference") (OtherBodyIndex :type Integer))
  (cast `/Game/Blueprints/BP_PlayerBall` OtherActor)
  (`self.DisableInput` (`GameplayStatics.GetPlayerController` 0))
  (`/Game/HUD/HUD_Principal.HideInteractionText` (`self.UIHUDREF`))
  (set `self.IsMoving` true)
  (set `self.MoveUp` false))

(event `InputAction|Action`
  (params (Key :type "Key Structure"))
  (:`Pressed`
    (if (not (`self.IsMoving`))
      (set `self.MoveUp` true)
      (set `self.IsMoving` true))))

(event `self.ReceiveTick`
  (params (DeltaSeconds :type "Float (single-precision)"))
  (bind (_returnvalue_x _returnvalue_y _returnvalue_z) (`KismetMathLibrary.BreakVector` (`self.K2_GetActorLocation`)))
  (bind (_returnvalue_x_2 _returnvalue_y_2 _returnvalue_z_2) (`KismetMathLibrary.BreakVector` (`self.K2_GetActorLocation`)))
  (bind _returnvalue (- _returnvalue_z (`self.SpeedOfPlatform`)))
  (bind _returnvalue_2 (+ _returnvalue_z_2 (`self.SpeedOfPlatform`)))
  (if (`self.IsMoving`)
    (if (`self.MoveUp`)
      (if (>= _returnvalue_2 (`self.UpLimit`))
        (set `self.IsMoving` false))
      (`self.K2_SetActorLocation` (`KismetMathLibrary.MakeVector` _returnvalue_x_2 _returnvalue_y_2 _returnvalue_2))
      (else
        (if (<= _returnvalue (`self.DownLimit`))
          (set `self.IsMoving` false))
        (`self.K2_SetActorLocation` (`KismetMathLibrary.MakeVector` _returnvalue_x _returnvalue_y _returnvalue))))))

(fn `UserConstructionScript`)